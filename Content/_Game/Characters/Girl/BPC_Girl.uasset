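; Player character Blueprint for the Girl, who runs, jumps and carries counts of milk, wool, yarn and cheese.
; Enhanced Input from IMC_Girl drives jumping and running, with movement only along the capsule's forward vector.
; On BeginPlay it creates the WPB_Objects HUD, and UpdateObjects writes the four counts into its text fields.
; FailedMilch and FailedWolle events play HUD animations signalling insufficient milk or wool.
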(event `EnhancedInput|/Game/_Game/Characters/Girl/Input/IA_Girl_Run`
  (params (ActionValue :type Boolean) (ElapsedSeconds :type "Float (double-precision)") (TriggeredSeconds :type "Float (double-precision)") (InputAction :type "InputAction Object Reference" :default "/Game/_Game/Characters/Girl/Input/IA_Girl_Run.IA_Girl_Run"))
  (:`Triggered`
    (`self.AddMovementInput` (`SceneComponent.GetForwardVector` (`self.CapsuleComponent`)) (`KismetMathLibrary.Conv_BoolToDouble` ActionValue))))

(event `EnhancedInput|/Game/_Game/Characters/Girl/Input/IA_Girl_Jump`
  (params (ActionValue :type Boolean) (ElapsedSeconds :type "Float (double-precision)") (TriggeredSeconds :type "Float (double-precision)") (InputAction :type "InputAction Object Reference" :default "/Game/_Game/Characters/Girl/Input/IA_Girl_Jump.IA_Girl_Jump"))
  (:`Triggered`
    (`self.Jump`))
  (:`Completed`
    (`self.StopJumping`)))

(event `self.ReceiveBeginPlay`
  ; UI in Level anzeigen
  (`EnhancedInputSubsystemInterface.AddMappingContext` (pcsubsystem `EnhancedInputLocalPlayerSubsystem` (`GameplayStatics.GetPlayerController` 0)) "/Game/_Game/Characters/Girl/Input/IMC_Girl.IMC_Girl" 1 (struct))
  (bind _returnvalue (`|CreateWidget` "/Game/_Game/UI/WPB_Objects.WPB_Objects_C"))
  (bind _output_get (set `self.UI_Objects` _returnvalue))
  (`UserWidget.AddToViewport` _output_get 0)
  (`self.UpdateObjects`))

(event `FailedMilch`
  ; Animation Abspielen wenn zu Wenig Ausgangsmaterial
  (`UserWidget.PlayAnimation` (stale `self.ReceiveBeginPlay` _returnvalue) (`/Game/_Game/UI/WPB_Objects.FailedMilch` (stale `self.ReceiveBeginPlay` _returnvalue)) 0.0 1 "Forward" 1.0 false))

(event `FailedWolle`
  ; Animation Abspielen wenn zu Wenig Ausgangsmaterial
  (`UserWidget.PlayAnimation` (stale `self.ReceiveBeginPlay` _returnvalue) (`/Game/_Game/UI/WPB_Objects.FailedWolle` (stale `self.ReceiveBeginPlay` _returnvalue)) 0.0 1 "Forward" 1.0 false))

(fn `UpdateObjects`
  (bind _ui_objects (`self.UI_Objects`))
  (bind _ui_objects_2 (`self.UI_Objects`))
  ; Update UI
  (`TextBlock.SetText` (`/Game/_Game/UI/WPB_Objects.MilchCounter` _ui_objects_2) (`KismetTextLibrary.Conv_IntToText` (`self.Milch Current`)))
  (`TextBlock.SetText` (`/Game/_Game/UI/WPB_Objects.WolleCounter` _ui_objects_2) (`KismetTextLibrary.Conv_IntToText` (`self.Wolle Current`)))
  (`TextBlock.SetText` (`/Game/_Game/UI/WPB_Objects.GarnCounter` _ui_objects) (`KismetTextLibrary.Conv_IntToText` (`self.Garn Current`)))
  (`TextBlock.SetText` (`/Game/_Game/UI/WPB_Objects.KaseCounter` _ui_objects) (`KismetTextLibrary.Conv_IntToText` (`self.Kase Current`)))
  (return))

(fn `UserConstructionScript`)