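; Sheep AI character that roams at random and can be clicked to open an interaction menu.
; On BeginPlay it creates a collapsed interaction widget and starts a roam loop: move to a random reachable point nearby, pause, repeat, continuing only on successful moves.
; Its HoverTrigger swaps in a highlight material under the cursor.
; Clicking shows the widget and marks the player character as Occupied, unless it already is.
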(event `self.HoverTrigger.OnClicked`
  (params (TouchedComponent :type "PrimitiveComponent Object Reference") (ButtonPressed :type "Key Structure"))
  ; Interaktions Schaf Buttons Sichtbar
  (bind _asbp_top_down_character (cast `/Game/TopDown/Blueprints/BP_TopDownCharacter` (`GameplayStatics.GetPlayerCharacter` 0)))
  (if (not (`/Game/TopDown/Blueprints/BP_TopDownCharacter.Occupied` _asbp_top_down_character))
    (`Widget.SetVisibility` (stale `self.ReceiveBeginPlay` _returnvalue) "Visible")
    (set `/Game/TopDown/Blueprints/BP_TopDownCharacter.Occupied` true _asbp_top_down_character)))

(event `self.ReceiveBeginPlay`
  ; WB Schaf Interaktion ins Level
  (bind _returnvalue (`|CreateWidget` "/Game/_Game/UI/WBP_InteractionSheep.WBP_InteractionSheep_C"))
  (`Widget.SetVisibility` _returnvalue "Collapsed")
  (`UserWidget.AddToViewport` _returnvalue 0)
  (`self.Random Roam`))

(event `Random Roam`
  ; Schafe random laufen können
  (set `CharacterMovementComponent.MaxWalkSpeed` 200.0 (`self.CharacterMovement`))
  (`|AIMoveTo` self (`NavigationSystemV1.K2_GetRandomReachablePointInRadius` (`self.K2_GetActorLocation`) 2500.0 null null) null
    (:`OnSuccess`
      (`KismetSystemLibrary.RetriggerableDelay` 5.0)
      (`self.Random Roam`))))

(event `self.HoverTrigger.OnBeginCursorOver`
  (params (TouchedComponent :type "PrimitiveComponent Object Reference"))
  ; Farbe bei Hovern ändern
  (`PrimitiveComponent.SetMaterial` (`self.Mesh`) 0 "/Game/_Game/Environment/Materials/M_Highlight.M_Highlight"))

(event `self.HoverTrigger.OnEndCursorOver`
  (params (TouchedComponent :type "PrimitiveComponent Object Reference"))
  ; Farbe bei Hovern ändern
  (`PrimitiveComponent.SetMaterial` (`self.Mesh`) 0 "/Game/_Game/Characters/Sheep/M_sheep.M_sheep"))

(fn `UserConstructionScript`)